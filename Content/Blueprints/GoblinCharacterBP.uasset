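; GoblinCharacterBP is a goblin character that also relays second-player keyboard input to another character.
; On BeginPlay it caches Player2 from ProjectCGameMode, then spawns a HurtBoxActorBP, snap-attaches it to itself and becomes its owner.
; The p2 move, jump and two attack inputs call matching P2Keyboard functions on that Player2 reference, with validity checks on all but jump release.
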(event Collision|EventActorBeginOverlap
  (params (OtherActor :type Actor%20Object%20Reference)))

(event EventTick
  (params (DeltaSeconds :type Float%20%28single-precision%29)))

(event EventBeginPlay
  (bind _self self)
  (bind _asproject_cgame_mode (Utilities|Casting|CastToProjectCGameMode (Game|GetGameMode)))
  (Variables|Default|Setplayer2ref (Variables|/Script/ProjectC.ProjectCGameMode|Getplayer2 _asproject_cgame_mode))
  (bind _returnvalue (Game|SpawnActorfromClass "/Game/Blueprints/hurtBoxActorBP.hurtBoxActorBP_C" (Transformation|GetActorTransform (Class|PawnMovementComponent|GetPawnOwner (Variables|Character|GetCharacterMovement))) "Undefined" 0 0))
  (bind _output_get (Variables|Default|Sethurtbox _returnvalue))
  (Transformation|AttachActorToActor _output_get _self "None" "SnapToTarget" "SnapToTarget" "SnapToTarget" true)
  (Actor|SetOwner _output_get _self))

(event Input|ActionEvents|InputActionp2Jump
  (params (Key :type Key%20Structure :default "None"))
  (bind _player2ref (Variables|Default|Getplayer2ref))
  (:Pressed
    (Utilities|IsValid _player2ref
      (:Is%20Valid
        (Class|ProjectCCharacter|P2KeyboardJump _player2ref))))
  (:Released
    (Class|ProjectCCharacter|P2KeyboardStopJumping _player2ref)))

(event Input|ActionEvents|InputActionp2attack1
  (params (Key :type Key%20Structure :default "None"))
  (bind _player2ref (Variables|Default|Getplayer2ref))
  (:Pressed
    (Utilities|IsValid _player2ref
      (:Is%20Valid
        (Class|ProjectCCharacter|P2KeyboardAttack1 _player2ref)))))

(event Input|ActionEvents|InputActionp2Jump
  (params (Key :type Key%20Structure :default "None")))

(event Input|ActionEvents|InputActionp2attack2
  (params (Key :type Key%20Structure :default "None"))
  (bind _player2ref (Variables|Default|Getplayer2ref))
  (:Pressed
    (Utilities|IsValid _player2ref
      (:Is%20Valid
        (Class|ProjectCCharacter|P2KeyboardAttack2 _player2ref)))))

(event Input|AxisEvents|InputAxisp2MoveRight
  (params (AxisValue :type Float%20%28single-precision%29))
  (bind _player2ref (Variables|Default|Getplayer2ref))
  (Utilities|IsValid _player2ref
    (:Is%20Valid
      (Class|ProjectCCharacter|P2KeyboardMoveRight _player2ref AxisValue))))

(fn ConstructionScript)