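; Game mode for a two-player fighting match that spawns both fighters, runs the round timer and picks a winner.
; BeginPlay spawns fighters at PlayerStarts by P1 tag, both using the game instance's character class, cross-links them, flips Player2 and shows healthbars.
; Tick counts down and checks for zero health or, at timeout, higher health, then shows an end widget.
; A timeout tie resets the clock without reactivating the timer.
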(event Custom|gameend
  (bind _player1 (Variables|Default|Getplayer1))
  (bind _player2 (Variables|Default|Getplayer2))
  (bind _playerhealth (Variables|/Script/ProjectC.ProjectCCharacter|GetplayerHealth _player1))
  (bind _playerhealth_2 (Variables|/Script/ProjectC.ProjectCCharacter|GetplayerHealth _player2))
  (if (Variables|Default|GetisTimerActive)
    (if (== (Variables|/Script/ProjectC.ProjectCCharacter|GetplayerHealth (Variables|Default|Getplayer1)) 0.0)
      (Variables|Default|SetWinner (Variables|Default|Getplayer2) :!label _label)
      (Class|ProjectCGameMode|DetermineWinner :!label _label_2)
      (bind _returnvalue (UserInterface|CreateWidget "/Game/Assets/widgets/NewWidgetBlueprint.NewWidgetBlueprint_C" (Game|GetPlayerController 0)))
      (UserInterface|Viewport|AddtoViewport _returnvalue 0)
      (elif (== (Variables|/Script/ProjectC.ProjectCCharacter|GetplayerHealth (Variables|Default|Getplayer2)) 0.0)
        (Variables|Default|SetWinner (Variables|Default|Getplayer1) :!label _label_3)
        (goto _label_2)))
    (elif (== _playerhealth _playerhealth_2)
      (Variables|Default|Setroundtime 1e+01)
      (elif (>= _playerhealth _playerhealth_2)
        (goto _label_3)
        (else
          (goto _label))))))

(event EventBeginPlay
  (bind _player1 (Variables|Default|Getplayer1))
  (bind _player2 (Variables|Default|Getplayer2))
  (bind _outactors (Actor|GetAllActorsOfClass "/Script/Engine.PlayerStart"))
  (for _array_element _outactors
    (CallFunction|SpawnPlayers _array_element))
  (if (Utilities|IsValid (Variables|Default|Getplayer1))
    (if (Utilities|IsValid (Variables|Default|Getplayer2))
      (Variables|/Script/ProjectC.ProjectCCharacter|Setotherplayer _player1 _player2)
      (Variables|/Script/ProjectC.ProjectCCharacter|Setotherplayer _player2 _player1)
      (Variables|/Script/ProjectC.ProjectCCharacter|Setisflipped _player2 true)
      (Variables|Default|SetisTimerActive true)
      (bind _returnvalue (UserInterface|CreateWidget "/Game/Assets/widgets/Healthbar.Healthbar_C" (Game|GetPlayerController 0)))
      (UserInterface|Viewport|AddtoViewport _returnvalue 0))))

(event EventTick
  (params (DeltaSeconds :type Float%20%28single-precision%29))
  (if (Variables|Default|GetisTimerActive)
    (if (>= (- (Variables|Default|Getroundtime) DeltaSeconds) 0.0)
      (Variables|Default|Setroundtime (- (Variables|Default|Getroundtime) DeltaSeconds))
      (else
        (Variables|Default|Setroundtime 0.0)
        (Variables|Default|SetisTimerActive false)))
    (CallFunction|Gameend)))

(fn ConstructionScript)

(fn SpawnPlayers
  (params (Object :type Actor%20Object%20Reference))
  (bind _returnvalue (Transformation|GetActorTransform Object))
  (bind _asplayer_start (Utilities|Casting|CastToPlayerStart Object))
  (if (Utilities|Name|Equal(Name) (Variables|/Script/Engine.PlayerStart|GetPlayerStartTag _asplayer_start) "P1")
    (bind _characterreference (CallFunction|DetermineCharacterClass (Transformation|GetActorTransform Object) Object))
    (bind _output_get (Variables|Default|Setplayer1 _characterreference))
    (Development|PrintString (Utilities|GetDisplayName _output_get))
    (Pawn|Possess (Game|GetPlayerController 0) _characterreference)
    (else
      (bind _returnvalue_2 (Game|SpawnActorfromClass "/Script/ProjectC.BasePlayerController" _returnvalue "Undefined" 0 0))
      (bind _characterreference_2 (CallFunction|DetermineCharacterClass _returnvalue Object))
      (bind _output_get_2 (Variables|Default|Setplayer2 _characterreference_2))
      (Development|PrintString (Utilities|GetDisplayName _output_get_2))
      (Pawn|Possess _returnvalue_2 _characterreference_2))))

(fn DetermineCharacterClass
  (params (transform :type Transform) (actor :type Actor%20Object%20Reference))
  (bind _asbase_game_instance (Utilities|Casting|CastToBaseGameInstance (Game|GetGameInstance)))
  (switch Utilities|FlowControl|Switch|SwitchonECharacterClass (Variables|/Script/ProjectC.BaseGameInstance|GetcharacterClass _asbase_game_instance)
    (:VE_Default
      (bind _returnvalue (Game|SpawnActorfromClass "/Game/Blueprints/BasicCharacterBP.BasicCharacterBP_C" transform "Undefined" actor 0))
      (return _returnvalue))
    (:VE_Samurai
      (bind _returnvalue_2 (Game|SpawnActorfromClass "/Game/Blueprints/SamuraiCharacterBP.SamuraiCharacterBP_C" transform "Undefined" actor 0))
      (return _returnvalue_2))
    (:VE_Goblin
      (bind _returnvalue_3 (Game|SpawnActorfromClass "/Game/Blueprints/GoblinCharacterBP.GoblinCharacterBP_C" transform "Undefined" actor 0))
      (return _returnvalue_3))))