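; Hitbox actor for a two-player combat game that damages the opponent of the player who owns it.
; SpawnHitbox sets a display material by hitbox type (proximity, strike or hurtbox), moves and hides the display, then runs CheckCollision.
; CheckCollision finds the owner's side through the game mode and does a one-time overlap test against the other player's hurtbox, applying HitboxDamage regardless of type.
; Debug prints remain throughout.
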(event Custom|SpawnHitbox
  (switch Utilities|FlowControl|Switch|SwitchonEHitboxEnum (Variables|Default|GethitboxType)
    (:HB_PROXIMITY
      (Rendering|Material|SetMaterial (Variables|Default|GetHitboxDisplay) 0 "/Game/materials/yellow.yellow"))
    (:HB_STRIKE
      (Rendering|Material|SetMaterial (Variables|Default|GetHitboxDisplay) 0 "/Game/materials/yellow1.yellow1"))
    (:HB_HURTBOX
      (Rendering|Material|SetMaterial (Variables|Default|GetHitboxDisplay) 0 "/Game/materials/yellow2.yellow2")))
  (Transformation|SetWorldLocation (Variables|Default|GetHitboxDisplay) (Variables|Default|Gethitboxlocation) false false)
  (Rendering|SetVisibility (Variables|Default|GetHitboxDisplay) false false)
  (CallFunction|CheckCollision))

(event Custom|CheckCollision
  (bind _basegamemodereference (Variables|Default|GetBaseGamemodeReference))
  (bind _basegamemodereference_2 (Variables|Default|GetBaseGamemodeReference))
  (bind _player2 (Variables|/Script/ProjectC.ProjectCGameMode|Getplayer2 _basegamemodereference))
  (bind _player1 (Variables|/Script/ProjectC.ProjectCGameMode|Getplayer1 _basegamemodereference_2))
  (bind _isplayer1 (CallFunction|Determineplayer))
  (if _isplayer1
    (Development|PrintString "Hello")
    (Utilities|IsValid _player2
      (:Is%20Valid
        (if (Collision|IsOverlappingActor (Variables|/Script/ProjectC.ProjectCCharacter|Gethurtbox _player2) :!class /Script/Engine.Actor)
          (Class|ProjectCCharacter|TakeDamage _player2 (Variables|Default|GethitboxDamage)))))
    (else
      (Development|PrintString (Utilities|GetDisplayName _player1))
      (Utilities|IsValid _player1
        (:Is%20Valid
          (if (Collision|IsOverlappingActor (Variables|/Script/ProjectC.ProjectCCharacter|Gethurtbox _player1) :!class /Script/Engine.Actor)
            (Class|ProjectCCharacter|TakeDamage _player1 (Variables|Default|GethitboxDamage))))))))

(event EventBeginPlay)

(event Collision|EventActorBeginOverlap
  (params (OtherActor :type Actor%20Object%20Reference)))

(event EventTick
  (params (DeltaSeconds :type Float%20%28single-precision%29)))

(fn ConstructionScript)

(fn Determineplayer
  (bind _self self)
  (bind _returnvalue (Components|GetOwner _self))
  (bind _asproject_cgame_mode (Utilities|Casting|CastToProjectCGameMode (Game|GetGameMode)))
  (bind _output_get (Variables|Default|SetBaseGamemodeReference _asproject_cgame_mode))
  (Development|PrintString (Utilities|GetDisplayName (Variables|/Script/ProjectC.ProjectCGameMode|Getplayer1 _output_get)))
  (Development|PrintString (Utilities|GetDisplayName _returnvalue))
  (if (== (Variables|/Script/ProjectC.ProjectCGameMode|Getplayer1 _output_get) _returnvalue)
    (return true)
    (else
      (return false))))